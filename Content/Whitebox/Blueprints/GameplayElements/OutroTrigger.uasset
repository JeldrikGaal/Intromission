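; OutroTrigger is a trigger actor that plays the game's ending sequence when player 0's pawn first overlaps it.
; A DoOnce gates the chain, which waits briefly, then plays a flashlight sound cue, shows OutroWidget, starts MediaSound and calls DisableInput on itself for the player controller.
; A long fixed Delay, rather than any media-finished event, then times the call to QuitGame.
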(event Collision|EventActorBeginOverlap
  (params (OtherActor :type Actor%20Object%20Reference))
  (bind _returnvalue (Game|GetPlayerController 0))
  (if (== OtherActor (Game|Player|GetPlayerPawn 0))
    (Utilities|FlowControl|DoOnce false
      (:Completed
        (Utilities|FlowControl|Delay 24.0)
        (Audio|PlaySound2D "/Game/Whitebox/Sound/CUEs/Flaschlight_Cue.Flaschlight_Cue" 1.0 1.0 0.0 0 0)
        (bind _returnvalue_2 (UserInterface|CreateWidget "/Game/Whitebox/Blueprints/UI/AudioWalks/OutroWidget.OutroWidget_C"))
        (UserInterface|Viewport|AddtoViewport _returnvalue_2 0)
        (CameraShake|Start (Variables|Default|GetMediaSound))
        (Input|DisableInput _returnvalue)
        (Utilities|FlowControl|Delay 313.0)
        (Game|QuitGame _returnvalue "Quit" false)))))

(fn ConstructionScript)