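; Test player state that runs timed dialogue subtitles and story-text progression.
; ShowDialoge gates two dialogues on predecessors, marks the caller's entry triggered, then HelpEvents advances lines by re-arming timers between start and end sounds.
; Completion records the dialogue number and, for certain dialogues, reveals a named InWorldText actor.
; Separately, Step moves an index through StoryEntry actors attached to "--STORY--", showing each through a duration-scaled Timeline.
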(event Custom|ShowDialoge
  (params (Text :type Array%20of%20Strings) (DialogNumber :type Integer) (Time :type Array%20of%20Floats%20%28single-precision%29) (text_field :type String) (callingActor :type Actor%20Object%20Reference) (index :type Integer) (ana :type Array%20of%20Booleans))
  (bind _currenttextindex (Variables|Default|GetcurrentTextIndex))
  ;[1 1 1] SpecialCases 11 + 12
  (if (== DialogNumber 11)
    (if (Utilities|Array|ContainsItem (Variables|Default|GetcompletedDialoges) 10)
      (Variables|Default|SetcurrentDialog DialogNumber :!label _label)
      (bind _asdialog (Utilities|Casting|CastToDialog callingActor)
        (:then
          (Utilities|Array|SetArrayElem (Variables|/Game/Whitebox/Blueprints/GameplayElements/Dialog.Dialog_C|GetdialogList _asdialog) index (Utilities|Struct|Makedialog_object (.text (Utilities|Struct|Breakdialog_object (Utilities|Array|Get(acopy) (Variables|/Game/Whitebox/Blueprints/GameplayElements/Dialog.Dialog_C|GetdialogList _asdialog) index))) (.dialog_number (Utilities|Struct|Breakdialog_object (Utilities|Array|Get(acopy) (Variables|/Game/Whitebox/Blueprints/GameplayElements/Dialog.Dialog_C|GetdialogList _asdialog) index))) (.time (Utilities|Struct|Breakdialog_object (Utilities|Array|Get(acopy) (Variables|/Game/Whitebox/Blueprints/GameplayElements/Dialog.Dialog_C|GetdialogList _asdialog) index))) (.interactable_name (Utilities|Struct|Breakdialog_object (Utilities|Array|Get(acopy) (Variables|/Game/Whitebox/Blueprints/GameplayElements/Dialog.Dialog_C|GetdialogList _asdialog) index))) (.text_object_optional (Utilities|Struct|Breakdialog_object (Utilities|Array|Get(acopy) (Variables|/Game/Whitebox/Blueprints/GameplayElements/Dialog.Dialog_C|GetdialogList _asdialog) index))) true (.isAnnaText (Utilities|Struct|Breakdialog_object (Utilities|Array|Get(acopy) (Variables|/Game/Whitebox/Blueprints/GameplayElements/Dialog.Dialog_C|GetdialogList _asdialog) index))))))
        (:CastFailed
          _))
      (Audio|PlaySoundatLocation "/Game/Whitebox/Sound/WalkieTalkie/dialoguestart.dialoguestart" (Transformation|GetActorLocation (Game|Player|GetPlayerPawn 0)) "0, 0, 0" 1.0 1.0 0.0 0 0 0)
      (Utilities|FlowControl|Delay 0.2)
      (Variables|Default|Setana (Utilities|Array|Get(acopy) ana (Variables|Default|GetcurrentTextIndex)))
      (Variables|Default|SetcurrentText (Utilities|Array|Get(acopy) Text))
      (Math|Integer|IncrementInt _currenttextindex
        (:%20%20
          (bind _returnvalue (Utilities|Time|SetTimerbyEvent (delegate Custom|HelpEvents) (Utilities|Array|Get(acopy) Time _currenttextindex)))
          (Variables|Default|SetTimer _returnvalue))))
    (elif (== DialogNumber 12)
      (if (Utilities|Array|ContainsItem (Variables|Default|GetcompletedDialoges) 11)
        (goto _label))
      (else
        (goto _label)))))

(event Custom|StepEvent
  (bind _asstory_entry (Utilities|Casting|CastToStoryEntry (Utilities|Array|Get(acopy) (Variables|Default|GetStoryElements) (- (- (Utilities|Array|Length (Variables|Default|GetStoryElements)) 1) (Variables|Default|Getindex)))))
  (Variables|Default|SetcurrentText (Variables|/Game/Whitebox/Blueprints/GameplayElements/StoryEntry.StoryEntry_C|GetText _asstory_entry))
  (Components|Timeline|SetPlayRate (Variables|Default|GetTimeline_0) (/ 1.0 (Variables|/Game/Whitebox/Blueprints/GameplayElements/StoryEntry.StoryEntry_C|GetTime _asstory_entry)))
  (Timeline|Timeline_0 PlayFromStart
    (:Finished
      (Variables|Default|SetcurrentText ""))))

(event Custom|HelpEvents
  (Variables|Default|SetcurrentText "")
  (Utilities|FlowControl|Delay 0.2)
  (Audio|PlaySoundatLocation "/Game/Whitebox/Sound/WalkieTalkie/dialogend.dialogend" (Transformation|GetActorLocation (Game|Player|GetPlayerPawn 0)) "0, 0, 0" 1.0 1.0 0.0 0 0 0)
  (if (== (Variables|Default|GetcurrentTextIndex) (Utilities|Array|Length (stale Custom|ShowDialoge Text)))
    (Utilities|Array|Add (Variables|Default|GetcompletedDialoges) (stale Custom|ShowDialoge DialogNumber))
    (Variables|Default|SetcurrentTextIndex 0)
    (Variables|Default|SetcurrentText "")
    (Utilities|Time|PauseTimerbyHandle (Variables|Default|GetTimer))
    (if (Math|Boolean|ORBoolean (== (Variables|Default|GetcurrentDialog) 8) (== (Variables|Default|GetcurrentDialog) 3) (== (Variables|Default|GetcurrentDialog) 9))
      (bind _actor (Utilities|GetActorbyName (stale Custom|ShowDialoge text_field))
        (:End
          (bind _asin_world_text (Utilities|Casting|CastToInWorldText _actor))
          (Default|ShowText _asin_world_text))))
    (Variables|Default|SetcurrentDialog 0)
    (else
      (Variables|Default|SetcurrentText (Utilities|Array|Get(acopy) (stale Custom|ShowDialoge Text) (Variables|Default|GetcurrentTextIndex)))
      (Variables|Default|Setana (Utilities|Array|Get(acopy) (stale Custom|ShowDialoge ana) (Variables|Default|GetcurrentTextIndex)))
      (Math|Integer|IncrementInt (Variables|Default|GetcurrentTextIndex)
        (:%20%20
          (bind _returnvalue (Utilities|Time|SetTimerbyEvent (delegate Custom|HelpEvents) (Utilities|Array|Get(acopy) (stale Custom|ShowDialoge Time) (Variables|Default|GetcurrentTextIndex))))
          (Variables|Default|SetTimer _returnvalue))))))

(event EventBeginPlay
  (bind _actor (Utilities|GetActorbyName "--STORY--")
    (:End
      (bind _output_get (Variables|Default|SetStoryElements (Actor|GetAttachedActors _actor true)))
      (for _array_element _output_get
        _))))

(fn ConstructionScript)

(fn Step
  (params (Calling%20Actor :type Actor%20Object%20Reference) (New%20Current%20State :type String) (Forward :type Boolean))
  (Variables|Default|SetlastAccess Calling%20Actor)
  (if (Utilities|Array|IsEmpty New%20Current%20State)
    _
    (else
      (Variables|Default|SetcurrentState New%20Current%20State)))
  (if Forward
    (Math|Integer|IncrementInt (Variables|Default|Getindex)
      (:%20%20
        _))
    (else
      (Math|Integer|DecrementInt (Variables|Default|Getindex)
        (:%20%20
          _))))
  (CallFunction|StepEvent))